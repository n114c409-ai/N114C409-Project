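; Parallax backdrop actor that shifts four background layers (far, mid and two near) as the player moves along X.
; BeginPlay records the player character's starting X, and each Tick calls UpdateParallax with no smoothing.
; UpdateParallax scales the player's X displacement by a per-layer factor and sets each component's relative location, using fixed Y offsets to stagger the layers in depth.
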(event EventBeginPlay
  (Variables|Default|SetPlayrtStartX (.X (Math|Vector|BreakVector (Transformation|GetActorLocation (Game|GetPlayerCharacter 0))))))

(event Collision|EventActorBeginOverlap
  (params (OtherActor :type Actor%20Object%20Reference)))

(event EventTick
  (params (DeltaSeconds :type Float%20%28single-precision%29))
  (CallFunction|UpdateParallax))

(fn ConstructionScript)

(fn UpdateParallax
  (Variables|Default|SetDeltaX (- (.X (Math|Vector|BreakVector (Transformation|GetActorLocation (Game|GetPlayerCharacter 0)))) (Variables|Default|GetPlayrtStartX)))
  (Utilities|FlowControl|Sequence
    (:then_0
      (Transformation|SetRelativeLocation (Variables|Default|GetSP_Far) (Math|Vector|MakeVector (+ (Variables|Default|GetXStart) (* (Variables|Default|GetDeltaX) (Variables|Default|GetFarBG))) (+ (Variables|Default|GetYStart) -2e+02) (Variables|Default|GetZStart)) false false))
    (:then_1
      (Transformation|SetRelativeLocation (Variables|Default|GetSP_Mid) (Math|Vector|MakeVector (+ (Variables|Default|GetXStart) (* (Variables|Default|GetDeltaX) (Variables|Default|GetMidBG))) (+ (Variables|Default|GetYStart) -1e+02) (Variables|Default|GetZStart)) false false))
    (:then_2
      (Transformation|SetRelativeLocation (Variables|Default|GetSP_Near01) (Math|Vector|MakeVector (+ (Variables|Default|GetXStart) (* (Variables|Default|GetDeltaX) (Variables|Default|GetSP_Near_01))) (+ (Variables|Default|GetYStart) -5e+01) (Variables|Default|GetZStart)) false false))
    (:then_3
      (Transformation|SetRelativeLocation (Variables|Default|GetSP_Near02) (Math|Vector|MakeVector (+ (Variables|Default|GetXStart) (* (Variables|Default|GetDeltaX) (Variables|Default|GetSP_Near_02))) (Variables|Default|GetYStart) (Variables|Default|GetZStart)) false false))))